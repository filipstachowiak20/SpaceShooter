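; Player spaceship Blueprint that creates and updates the main HUD.
; On BeginPlay it creates the MainHud widget, adds it to the viewport and stores a reference.
; The UpdateHUD event writes force field, score and ammo values into the widget's text blocks, displaying 999 when ammo is zero.
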(event `self.ReceiveBeginPlay`
  (bind _returnvalue (`|CreateWidget` "/Game/Blueprints/Widgets/MainHud.MainHud_C"))
  (`UserWidget.AddToViewport` _returnvalue 0)
  (set `self.MainHUDRef` _returnvalue))

(event `self.UpdateHUD`
  (bind _mainhudref (`self.MainHUDRef`))
  (bind _ammo (`self.Ammo`))
  (`TextBlock.SetText` (`/Game/Blueprints/Widgets/MainHud.ScoreText_1` _mainhudref) (`KismetTextLibrary.Conv_DoubleToText` (`self.ForceField`) "HalfToEven" false true 1 324 0 1))
  (`TextBlock.SetText` (`/Game/Blueprints/Widgets/MainHud.ScoreText` _mainhudref) (`KismetTextLibrary.Conv_IntToText` (`self.Score`)))
  (`TextBlock.SetText` (`/Game/Blueprints/Widgets/MainHud.AmmoText` _mainhudref) (`KismetTextLibrary.Conv_IntToText` (`KismetMathLibrary.SelectInt` 999 _ammo (== _ammo 0)))))

(fn `UserConstructionScript`)